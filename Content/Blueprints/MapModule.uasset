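; MapModule is a map section actor that tracks which module the player and NPCs have entered.
; On BeginPlay it converts its first actor tag to an integer, passes it to InitModule and stores the result as its Module.
; When CharacterDetector is overlapped, it writes itself to the player character's Module variable or, for NPC_AI_2, to the CurrentModule blackboard key.
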(event OnComponentBeginOverlap(CharacterDetector)
  (params (OverlappedComponent :type Primitive%20Component%20Object%20Reference) (OtherActor :type Actor%20Object%20Reference) (OtherComp :type Primitive%20Component%20Object%20Reference) (OtherBodyIndex :type Integer) (bFromSweep :type Boolean) (SweepResult :type Hit%20Result%20Structure%20%28by%20ref%29))
  (bind _self self)
  (if (Actor|ActorHasTag OtherActor "Player")
    (bind _asbp_third_person_character (Utilities|Casting|CastToBP_ThirdPersonCharacter OtherActor))
    (Variables|/Game/ThirdPerson/Blueprints/BP_ThirdPersonCharacter.BP_ThirdPersonCharacter_C|SetModule _asbp_third_person_character _self)
    (else
      (bind _asnpc_ai_2 (Utilities|Casting|CastToNPC_AI_2 OtherActor))
      (AI|Components|Blackboard|SetValueasObject (AI|GetBlackboard (Pawn|GetController _asnpc_ai_2)) (Variables|Default|GetCurrentModule) _self))))

(event EventBeginPlay
  (bind _returnvalue (Class|UMMapModule|InitModule (Math|Conversions|ToInteger(Byte) (Utilities|String|ToString(Name) (Utilities|Array|Get(acopy) (Variables|Actor|GetTags))))))
  (Variables|Default|SetModule _returnvalue))

(fn ConstructionScript)