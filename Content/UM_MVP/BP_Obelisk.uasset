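; Obelisk Blueprint that appears to be a test bed for building skeletal animation at runtime.
; On BeginPlay it generates an animation sequence from a hard-coded timeline of rotation keys on Bone_001 for its skeletal mesh's asset and stores it.
; Holding primary select calls PlayMontage with no montage set and prints on completion.
; Nodes for playing an animation and printing a sequence-difference score against Bendy are left unwired.
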(event Input|EnhancedActionEvents|EnhancedInputActionIA_PrimarySelectHold
  (params (ActionValue :type Boolean) (ElapsedSeconds :type Float%20%28double-precision%29) (TriggeredSeconds :type Float%20%28double-precision%29) (InputAction :type Input%20Action%20Object%20Reference :default "/Game/UM_MVP/FirstPerson/Input/Actions/IA_PrimarySelectHold.IA_PrimarySelectHold"))
  (Animation|Montage|PlayMontage 0 0
    (:OnCompleted
      (Development|PrintString "Finished"))))

(event EventBeginPlay
  (|CallParentFunction)
  (bind _returnvalue (Class|UMAnimationProducer|CreateSequence (Utilities|Map|MakeMap "Bone_001" (Utilities|Struct|MakeUMJointTimeline (Utilities|Array|MakeArray (Utilities|Struct|MakeUMJointKey 0.0 (Math|Transform|MakeTransform "0, 0, 0" "0, 0, 0" "1.000000,1.000000,1.000000")) (Utilities|Struct|MakeUMJointKey 1.0 (Math|Transform|MakeTransform "0, 0, 0" "0.000000,90.000000,0.000000" "1.000000,1.000000,1.000000")) (Utilities|Struct|MakeUMJointKey 2.0 (Math|Transform|MakeTransform "0, 0, 0" "90.000000,0.000000,90.000000" "1.000000,1.000000,1.000000")) (Utilities|Struct|MakeUMJointKey 3.0 (Math|Transform|MakeTransform "0, 0, 0" "0.000000,0.000000,-90.000000" "1.000000,1.000000,1.000000"))) 0.0 0.0)) (.AsSkeletal%20Mesh (Utilities|Casting|CastToSkeletalMesh (Class|SkinnedMeshComponent|GetSkinnedAsset (Variables|Default|GetSkeletalMesh))))))
  (Variables|Default|SetSequence _returnvalue))

(fn ConstructionScript)